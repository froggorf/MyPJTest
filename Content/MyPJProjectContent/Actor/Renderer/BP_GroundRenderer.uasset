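; BP_GroundRenderer is an actor that builds an isometric-style tiled ground from static mesh components in its construction script.
; Two diagonal step vectors in the YZ plane, derived from angle and length variables, position a fixed nested-loop grid of scaled, rotated tiles.
; Each tile gets a dynamic floor material instance whose tileset parameters pick the tile, switching row partway along the right-down axis.
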(event EventBeginPlay
  (for _array_element 0
    _))

(event Collision|EventActorBeginOverlap
  (params (OtherActor :type Actor%20Object%20Reference)))

(event EventTick
  (params (DeltaSeconds :type Float%20%28single-precision%29)))

(fn ConstructionScript
  (bind _x_rightdown_tileoffsetlength (Variables|Default|GetX%28RightDown%29TileOffsetLength))
  (bind _y_leftdown_tileoffsetlength (Variables|Default|GetY%28LeftDown%29TileOffsetLength))
  (bind _y_leftdown_angled (Variables|Default|GetY%28LeftDown%29AngleD))
  (LocalVariables|SetRightDownOffset (Math|Vector|MakeVector 0.0 (* _x_rightdown_tileoffsetlength (Math|Trig|Sin(Degrees) (Variables|Default|GetX%28RightDown%29AngleD))) (* _x_rightdown_tileoffsetlength (Math|Trig|Cos(Degrees) (Variables|Default|GetX%28RightDown%29AngleD)) -1.0)))
  (LocalVariables|SetLeftDownOffset (Math|Vector|MakeVector 0.0 (* _y_leftdown_tileoffsetlength (Math|Trig|Sin(Degrees) _y_leftdown_angled) -1.0) (* _y_leftdown_tileoffsetlength (Math|Trig|Cos(Degrees) _y_leftdown_angled) -1.0)))
  (for _index (range 0 50) ; 우하단 - x
    (for _index_2 (range 0 30) ; 좌하단 - y
      (bind _returnvalue (AddComponent|AddStaticMeshComponent true))
      (Transformation|AttachComponentToComponent _returnvalue (Variables|Default|GetScene) "None" "KeepRelative" "KeepRelative" "KeepRelative" true)
      (Transformation|SetRelativeTransform _returnvalue (Math|Transform|MakeTransform (+ (* (LocalVariables|GetLeftDownOffset) _index_2) (* (LocalVariables|GetRightDownOffset) _index)) "0.000000,0.000000,0.000000" "1.000000,1.330000,0.670000") false false)
      (Transformation|AddWorldRotation _returnvalue "0.000000,90.000000,90.000000" false false)
      (bind _returnvalue_2 (Rendering|Material|CreateDynamicMaterialInstance _returnvalue 0 (Variables|Default|GetFloorMaterialInstance) "None" :!class /Script/Engine.PrimitiveComponent))
      (Rendering|Material|SetScalarParameterValue _returnvalue_2 "TileSetX" 0.0 :!class /Script/Engine.MaterialInstanceDynamic)
      (Rendering|Material|SetScalarParameterValue _returnvalue_2 "TileSetY" (Math|Float|SelectFloat 0.0 2.0 (> _index 25)) :!class /Script/Engine.MaterialInstanceDynamic)
      (Rendering|Material|SetScalarParameterValue _returnvalue_2 "MaxTileSetY" 1e+01 :!class /Script/Engine.MaterialInstanceDynamic))))